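; Player-controlled pool cue that aims and strikes the cue ball in a billiards game.
; It attaches to the cue ball after BeginPlay, so axis input rotates the ball to aim with clamped pitch, while Left Shift offsets the cue within limits.
; Left click detaches the cue and applies a one-time force to the ball along the tip-to-ball direction.
; Tab toggles a blended view between the top camera and the cue.
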(event `self.ReceiveBeginPlay`
  (`KismetSystemLibrary.Delay` 0.2)
  (`self.K2_SetActorLocationAndRotation` (-640.0 0.0 110.0) (struct :`Pitch` -10.0))
  (`self.K2_AttachToActor` (`self.CueBall`) "None" "KeepRelative" "KeepRelative" "KeepWorld" true))

(event `self.ReceiveTick`
  (params (DeltaSeconds :type "Float (single-precision)"))
  (if (or (!= (`self.GetInputAxisKeyValue`) 0.0) (!= 0.0 (`self.GetInputAxisKeyValue`)))
    (if (`self.HasShot`)
      _
      (elif (`PlayerController.IsInputKeyDown` (`GameplayStatics.GetPlayerController` 0) "LeftShift")
        (`self.K2_SetActorRelativeLocation` (`KismetMathLibrary.MakeVector` (.x (+ (`KismetMathLibrary.MakeVector` 0.0 (`self.GetInputAxisKeyValue`) (`self.GetInputAxisKeyValue`)) (`SceneComponent.RelativeLocation` (`self.DefaultSceneRoot`)))) (`KismetMathLibrary.FClamp` (.y (+ (`KismetMathLibrary.MakeVector` 0.0 (`self.GetInputAxisKeyValue`) (`self.GetInputAxisKeyValue`)) (`SceneComponent.RelativeLocation` (`self.DefaultSceneRoot`)))) -45.0 45.0) (`KismetMathLibrary.FClamp` (.z (+ (`KismetMathLibrary.MakeVector` 0.0 (`self.GetInputAxisKeyValue`) (`self.GetInputAxisKeyValue`)) (`SceneComponent.RelativeLocation` (`self.DefaultSceneRoot`)))) 75.0 180.0)))
        (else
          (`self.K2_AddActorLocalRotation` (`self.CueBall`) (`KismetMathLibrary.MakeRotator` 0.0 (`self.GetInputAxisKeyValue`) (`self.GetInputAxisKeyValue`)) false false)
          (`self.K2_SetActorRotation` (`self.CueBall`) (`KismetMathLibrary.MakeRotator` 0.0 (`KismetMathLibrary.FClamp` (.pitch (`self.K2_GetActorRotation` (`self.CueBall`))) -45.0 10.0) (.yaw (`self.K2_GetActorRotation` (`self.CueBall`)))) false))))))

(event `Key|LeftMouseButton`
  (params (Key :type "Key Structure"))
  (:`Pressed`
    (if (not (`self.HasShot`))
      (set `self.HasShot` true)
      (`self.K2_DetachFromActor` "KeepWorld" "KeepWorld" "KeepWorld")
      (`PrimitiveComponent.AddForce` (`/Game/Blueprints/CueBall.Sphere` (`self.CueBall`)) (* (`KismetMathLibrary.Normal` (- (`SceneComponent.K2_GetComponentLocation` (`self.Tip`)) (`self.K2_GetActorLocation` (`self.CueBall`)))) -40000.0) "None" false))))

(event `Key|Tab`
  (params (Key :type "Key Structure"))
  ;[1 1 1] Switch Camera
  (:`Pressed`
    (`/Engine/EditorBlueprintResources/StandardMacros.FlipFlop`
      (:`A`
        (`PlayerController.SetViewTargetWithBlend` (`GameplayStatics.GetPlayerController` 0) (`self.TopCamera`) 1.0 "VTBlend_Linear" 0.0 true))
      (:`B`
        (`PlayerController.SetViewTargetWithBlend` (`GameplayStatics.GetPlayerController` 0) self 1.0 "VTBlend_Linear" 0.0 true)))))

(fn `RotateAround`
  (params (Center :type "Vector Structure") (Rotation :type "Rotator Structure") (Distance :type "Float (double-precision)"))
  (returns (OutPoint :type "Vector Structure"))
  (return (+ Center (* (`KismetMathLibrary.GetForwardVector` Rotation) Distance))))

(fn `UserConstructionScript`)